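; BP_AI_Car is an AI-driven sports car that follows a spline track at constant full throttle.
; Each tick it fetches all Path actors and steers along the first one's spline.
; GetPath projects a look-ahead point along the nearest spline tangent, snaps it to the spline and maps the yaw error to clamped steering input.
; Spline queries use local space despite world-space car positions.
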(event `self.ReceiveBeginPlay`
  (`WheeledVehicleMovementComponent.SetThrottleInput` (`self.VehicleMovement`) 1.0))

(event `self.ReceiveTick`
  (params (DeltaSeconds :type "Float (single-precision)"))
  (bind _outactors (`GameplayStatics.GetAllActorsOfClass` "/Game/AI/Path.Path_C"))
  (bind _steering (`self.Get Path` _outactors))
  (`WheeledVehicleMovementComponent.SetSteeringInput` (`self.VehicleMovement`) _steering))

(fn `Get Path`
  (params (Spline :type "Array of /Game/AI/Path Object Reference"))
  (returns (Steering :type "Float (double-precision)"))
  (bind _returnvalue (`self.K2_GetActorLocation`))
  (bind _spline (`/Game/AI/Path.Spline` (`|GetArrayItem` Spline)))
  (bind (_returnvalue_roll _returnvalue_pitch _returnvalue_yaw) (`KismetMathLibrary.BreakRotator` (`KismetMathLibrary.NormalizedDeltaRotator` (`KismetMathLibrary.FindLookAtRotation` _returnvalue (`SplineComponent.FindLocationClosestToWorldLocation` _spline (+ (* (`KismetMathLibrary.Normal` (`SplineComponent.FindTangentClosestToWorldLocation` _spline _returnvalue "Local")) 500.0) _returnvalue) "Local")) (`self.K2_GetActorRotation`))))
  (return (`KismetMathLibrary.MapRangeClamped` _returnvalue_yaw -90.0 90.0 -1.0 1.0)))

(fn `UserConstructionScript`)